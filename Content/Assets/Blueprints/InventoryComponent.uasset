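; Inventory component that stores an item list for its owner and shows it through a WBP_Inventory widget.
; Contents load asynchronously on BeginPlay and save on EndPlay to an SG_Inventory slot named from component and owner.
; Open fills a new widget from Contents, and Close copies the widget's contents back.
; TryAddItem delegates placement to a temporarily opened, transparent widget, then closes it and returns the amount that did not fit.
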(event `self.ReceiveBeginPlay`
  (bind _returnvalue (`KismetStringLibrary.Concat_StrStr` (`KismetSystemLibrary.GetObjectName` self) (`KismetSystemLibrary.GetObjectName` (`self.GetOwner`))))
  (`KismetSystemLibrary.PrintString` _returnvalue true true (struct :`R` 1.0 :`A` 1.0))
  (bind _returnvalue_2 (`GameplayStatics.DoesSaveGameExist` _returnvalue 0))
  (if _returnvalue_2
    (bind _savegame (`AsyncActionHandleSaveGame.AsyncLoadGameFromSlot` _returnvalue 0)
      (:`Completed`
        (bind _assg_inventory (cast `/Game/Assets/Blueprints/SG_Inventory` _savegame))
        (bind _output_get (set `self.SaveGameRef` _assg_inventory))
        (set `self.Contents` (`/Game/Assets/Blueprints/SG_Inventory.Contents` _output_get))))))

(event `self.ReceiveEndPlay`
  (params (EndPlayReason :type "EEndPlayReason Enum" :default "Destroyed"))
  (bind _returnvalue (`KismetStringLibrary.Concat_StrStr` (`KismetSystemLibrary.GetObjectName` self) (`KismetSystemLibrary.GetObjectName` (`self.GetOwner`))))
  (bind _returnvalue_2 (`GameplayStatics.DoesSaveGameExist` _returnvalue 0))
  (if _returnvalue_2
    (bind _savegame (`AsyncActionHandleSaveGame.AsyncLoadGameFromSlot` _returnvalue 0)
      (:`Completed`
        (bind _assg_inventory (cast `/Game/Assets/Blueprints/SG_Inventory` _savegame))
        (set `self.SaveGameRef` _assg_inventory)))
    (else
      (bind _returnvalue_3 (`GameplayStatics.CreateSaveGameObject` "/Game/Assets/Blueprints/SG_Inventory.SG_Inventory_C"))
      (set `self.SaveGameRef` _returnvalue_3)))
  (set `/Game/Assets/Blueprints/SG_Inventory.Contents` (`self.Contents`) (`self.SaveGameRef`))
  (`GameplayStatics.SaveGameToSlot` (`self.SaveGameRef`) _returnvalue 0))

(fn `Close`
  (`KismetArrayLibrary.Array_Clear` (`self.Contents`))
  (set `self.Contents` (`/Game/Assets/Blueprints/WBP_Inventory_Base.GetContents` (`self.InventoryRef`)))
  (`Widget.RemoveFromParent` (`self.InventoryRef`))
  (set `self.IsOpen` false))

(fn `Open`
  (`|ExecutionSequence`
    (:`then_0`
      (bind _returnvalue (`|CreateWidget` "/Game/Assets/Blueprints/WBP_Inventory.WBP_Inventory_C" (`GameplayStatics.GetPlayerController` 0) (`self.SlotNum`) (`self.ColumnNum`)))
      (bind _output_get (set `self.InventoryRef` _returnvalue))
      (`UserWidget.AddToViewport` _output_get 0)
      (`UserWidget.SetPositionInViewport` (`self.InventoryRef`) (/ (`WidgetLayoutLibrary.GetViewportSize`) (1.7 5.0)) false))
    (:`then_1`
      (for _array_element (`self.Contents`)
        (`/Game/Assets/Blueprints/WBP_Inventory_Base.TryAddItem` (`self.InventoryRef`) (break `/Game/Assets/Blueprints/S_InventoryContent` _array_element) (`.ItemNum_5_C4E68B7B427F4C84110582B05CC278AE` (break `/Game/Assets/Blueprints/S_InventoryContent` _array_element))))
      (set `self.IsOpen` true))))

(fn `TryAddItem`
  (params (ItemName :type Name) (ItemAmount :type Integer))
  (returns (ReminingNum :type Integer))
  (locals (TmpRemainingNum :type Integer))
  (bind _contents (`self.Contents`))
  (bind _inventoryref (`self.InventoryRef`))
  (`|ExecutionSequence`
    (:`then_0`
      (`self.Open`)
      (`Widget.SetRenderOpacity` _inventoryref 0.0)
      (bind _reminingnum (`/Game/Assets/Blueprints/WBP_Inventory_Base.TryAddItem` _inventoryref ItemName ItemAmount))
      (set `local.TmpRemainingNum` _reminingnum))
    (:`then_1`
      (`KismetArrayLibrary.Array_Set` _contents (`KismetArrayLibrary.Array_Length` _contents) (make `/Game/Assets/Blueprints/S_InventoryContent` ItemName (- ItemAmount (`local.TmpRemainingNum`))) true)
      (`self.Close`)
      (return (`local.TmpRemainingNum`)))))
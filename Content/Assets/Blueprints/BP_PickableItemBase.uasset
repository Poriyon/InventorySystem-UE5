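; Base pickable item actor that holds an item name and amount and offers them to any overlapping Character.
; The character's PickupItemMessage returns the leftover amount: zero expires the actor almost immediately, while a positive value becomes its new amount.
; UpdateObjectInfo sets the item data and, for dropped items, shrinks the actor, gives it a lifespan and launches its mesh with temporary physics.
; The launch impulse reuses the forward vector's X component for Z.
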(event `UpdateObjectInfo`
  (params (IsDropped :type Boolean) (ItemAmount :type Integer) (ItemName :type Name))
  (bind (_returnvalue_x _returnvalue_y) (`KismetMathLibrary.BreakVector` (* (`KismetMathLibrary.GetForwardVector` (`self.K2_GetActorRotation`)) 20000.0)))
  (set `self.ItemAmount` ItemAmount)
  (set `self.ItemName` ItemName)
  (if IsDropped
    (`|ExecutionSequence`
      (:`then_0`
        (`self.SetActorScale3D` (0.2 0.2 0.2))
        (`self.SetLifeSpan` 10.0)
        (`PrimitiveComponent.SetSimulatePhysics` (`self.StaticMesh`) true))
      (:`then_1`
        (`PrimitiveComponent.AddImpulse` (`self.StaticMesh`) (`KismetMathLibrary.MakeVector` _returnvalue_x _returnvalue_y _returnvalue_x) "None" false)
        (`KismetSystemLibrary.Delay` 5.0)
        (`PrimitiveComponent.SetSimulatePhysics` (`self.StaticMesh`) false)))))

(event `self.ReceiveActorBeginOverlap`
  (params (OtherActor :type "Actor Object Reference"))
  (bind _ascharacter (cast `Character` OtherActor))
  (bind _remainingnum (message `/Game/Assets/Blueprints/BPI_Player.PickupItem` _ascharacter (`self.ItemName`) (`self.ItemAmount`)))
  (if (== _remainingnum 0)
    (`self.SetLifeSpan` 0.1)
    (elif (> _remainingnum 0)
      (bind _output_get (set `self.ItemAmount` _remainingnum))
      ;[1 1 1] Debug
      (`KismetSystemLibrary.PrintString` (`KismetStringLibrary.Concat_StrStr` "CurrentAmount = " (`KismetStringLibrary.Conv_IntToString` _output_get))))))

(fn `UserConstructionScript`)